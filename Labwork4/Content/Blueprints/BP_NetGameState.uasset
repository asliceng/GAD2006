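; Game state Blueprint for a networked team match that drives the match timer and the end-of-round result screen.
; On begin play or restart it polls every fraction of a second until two players exist, then shows the timer widget and starts the countdown.
; On victory it compares the local player's team with the winner's to show a lose or named-winner message.
; The avatar won/lost notifications are left unconnected.
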(event `self.OnVictory`
  (for _array_element (`self.PlayerArray`)
    (bind _asnet_player_state (cast `NetPlayerState` _array_element))
    (bind (_data_nickname _data_customizationdata _data_teamid) (break `SPlayerInfo` (`NetPlayerState.Data` _asnet_player_state)))
    (switch `EPlayerTeam` _data_teamid))
  (`self.ShowResultMessage`))

(event `self.OnRestart`
  (`Widget.RemoveFromParent` (`self.Message Widget`))
  (if (>= (`KismetArrayLibrary.Array_Length` (`self.PlayerArray`)) 2) :!label _label
    (bind _returnvalue (`|CreateWidget` "/Game/Blueprints/UMG/W_Timer.W_Timer_C"))
    (`UserWidget.AddToViewport` _returnvalue 0)
    (`self.StartGameTimer`)
    (else
      (`KismetSystemLibrary.Delay` 0.2)
      (goto _label))))

(event `self.ReceiveBeginPlay`
  (goto _label))

(event `self.UpdateTimerDisplay`
  (`/Game/Blueprints/UMG/W_Timer.RemainingTime` (stale `self.OnRestart` _returnvalue) (`self.RemainingTime`)))

(fn `ShowResultMessage`
  (bind (_data_nickname _data_customizationdata _data_teamid) (break `SPlayerInfo` (`NetPlayerState.Data` (cast `NetPlayerState` (`Controller.PlayerState` (`GameplayStatics.GetPlayerController` 0)) :!pure true))))
  (bind _returnvalue (`self.GetPlayerStateByIndex` (`self.WinningPlayer`)))
  (bind (_nickname _customizationdata _teamid) (break `SPlayerInfo` (`NetPlayerState.Data` _returnvalue)))
  (bind _returnvalue_2 (`|CreateWidget` "/Game/Blueprints/UMG/W_GameResults.W_GameResults_C" null (select `bool` (`|EnumInequality` _data_teamid _teamid) :`false` (`|FormatText` "{name} WINS!" _nickname) :`true` "YOU LOSE!")))
  (bind _output_get (set `self.Message Widget` _returnvalue_2))
  (`UserWidget.AddToViewport` _output_get 0))

(fn `UserConstructionScript`)